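; Ghost trap actor that ragdolls a first-person or second-person player character when it enters the trigger box.
; On BeginPlay it sets itself as owner of its two GhostMine child actors.
; A valid overlap calls the character's Ragdoll, passing itself only to the first-person one, then prints a debug message, disables box collision and destroys the trap two ticks later.
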(event OnComponentBeginOverlap(Box)
  (params (OverlappedComponent :type Primitive%20Component%20Object%20Reference) (OtherActor :type Actor%20Object%20Reference) (OtherComp :type Primitive%20Component%20Object%20Reference) (OtherBodyIndex :type Integer) (bFromSweep :type Boolean) (SweepResult :type Hit%20Result%20Structure%20%28by%20ref%29))
  (bind _asbp_first_person_character (Utilities|Casting|CastToBP_FirstPersonCharacter OtherActor)
    (:then
      (Default|Ragdoll _asbp_first_person_character self))
    (:CastFailed
      (bind _asbp_second_person_character (Utilities|Casting|CastToBP_SecondPerson_Character OtherActor))
      (Default|Ragdoll _asbp_second_person_character)))
  (Development|PrintString "slippy :D")
  (Collision|SetCollisionEnabled (Variables|Default|GetBox) "NoCollision")
  (Utilities|FlowControl|DelayUntilNextTick)
  (Utilities|FlowControl|DelayUntilNextTick)
  (Actor|DestroyActor))

(event EventBeginPlay
  (Actor|SetOwner (Variables|/Script/Engine.ChildActorComponent|GetChildActor (Variables|Default|GetGhostMine1)) self)
  (Actor|SetOwner (Variables|/Script/Engine.ChildActorComponent|GetChildActor (Variables|Default|GetGhostMine)) self))

(fn ConstructionScript)