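; Pawn for a two-player tutorial or menu screen that shows a fixed camera view and moves both players on to the next level.
; BeginPlay points both player controllers at the MainMenuCamera actor and gives each a fade-in widget.
; Enter or gamepad Special Right fades both screens to black once, then opens NewMap after a short delay, while Escape quits.
; A custom event, not called here, adds a main menu widget per player.
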(event Custom|CustomEvent
  (Utilities|FlowControl|DelayUntilNextTick)
  (Utilities|FlowControl|Sequence
    (:then_0
      (bind _returnvalue (UserInterface|CreateWidget "/Game/UI/MainMenuWidget.MainMenuWidget_C" (Game|GetPlayerController 1)))
      (UserInterface|Viewport|AddtoPlayerScreen _returnvalue))
    (:then_1
      (bind _returnvalue_2 (UserInterface|CreateWidget "/Game/UI/MainMenuWidget.MainMenuWidget_C" (Game|GetPlayerController 0)))
      (UserInterface|Viewport|AddtoPlayerScreen _returnvalue_2))))

(event EventBeginPlay
  (Utilities|FlowControl|DelayUntilNextTick)
  (bind _outactors (Actor|GetAllActorsOfClass "/Game/Blueprints/MainMenuCamera.MainMenuCamera_C"))
  (for _array_element _outactors
    (Utilities|FlowControl|Sequence
      (:then_0
        (Game|Player|SetViewTargetwithBlend (Game|GetPlayerController 0) _array_element 0.0 "VTBlend_Linear" 0.0 false)
        (bind _returnvalue (UserInterface|CreateWidget "/Game/UI/FadeInFromBlack_WBP.FadeInFromBlack_WBP_C" (Game|GetPlayerController 0)))
        (UserInterface|Viewport|AddtoPlayerScreen _returnvalue))
      (:then_1
        (Game|Player|SetViewTargetwithBlend (Game|GetPlayerController 1) _array_element 0.0 "VTBlend_Linear" 0.0 false)
        (bind _returnvalue_2 (UserInterface|CreateWidget "/Game/UI/FadeInFromBlack_WBP.FadeInFromBlack_WBP_C" (Game|GetPlayerController 1)))
        (UserInterface|Viewport|AddtoPlayerScreen _returnvalue_2)))))

(event Input|KeyboardEvents|Enter
  (params (Key :type Key%20Structure :default "None"))
  (:Pressed
    (Utilities|FlowControl|DoOnce false
      (:Completed
        (Utilities|FlowControl|Sequence
          (:then_0
            (bind _returnvalue (UserInterface|CreateWidget "/Game/UI/FadeToBlack_WBP.FadeToBlack_WBP_C" (Game|GetPlayerController 0)))
            (UserInterface|Viewport|AddtoPlayerScreen _returnvalue))
          (:then_1
            (bind _returnvalue_2 (UserInterface|CreateWidget "/Game/UI/FadeToBlack_WBP.FadeToBlack_WBP_C" (Game|GetPlayerController 1)))
            (UserInterface|Viewport|AddtoPlayerScreen _returnvalue_2))
          (:then_2
            (Utilities|FlowControl|Delay 1.51)
            (Game|OpenLevel(byObjectReference) "/Game/wilFolder/NewMap.NewMap")))))))

(event Input|GamepadEvents|GamepadSpecialRight
  (params (Key :type Key%20Structure :default "None"))
  (:Pressed
    (Utilities|FlowControl|DoOnce false
      (:Completed
        (Utilities|FlowControl|Sequence
          (:then_0
            (bind _returnvalue (UserInterface|CreateWidget "/Game/UI/FadeToBlack_WBP.FadeToBlack_WBP_C" (Game|GetPlayerController 0)))
            (UserInterface|Viewport|AddtoPlayerScreen _returnvalue))
          (:then_1
            (bind _returnvalue_2 (UserInterface|CreateWidget "/Game/UI/FadeToBlack_WBP.FadeToBlack_WBP_C" (Game|GetPlayerController 1)))
            (UserInterface|Viewport|AddtoPlayerScreen _returnvalue_2))
          (:then_2
            (Utilities|FlowControl|Delay 1.51)
            (Game|OpenLevel(byObjectReference) "/Game/wilFolder/NewMap.NewMap")))))))

(event Input|KeyboardEvents|Escape
  (params (Key :type Key%20Structure :default "None"))
  (:Pressed
    (Game|QuitGame 0 "Quit" false)))

(fn ConstructionScript)