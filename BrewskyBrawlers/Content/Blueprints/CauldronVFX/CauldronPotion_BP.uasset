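; CauldronPotion_BP is a cauldron potion visual that rises and grows from zero to its placed scale on BeginPlay.
; The game mode's PotionsLeft picks which of two timelines drives that rise, with a separate one used at zero.
; Another timeline restarts itself to spin the potion mesh continuously.
; RedTeamPotion selects the material and delayed red or green particle burst, and red also swaps to the EvilPotion mesh.
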(event EventBeginPlay
  (bind _potionmesh (Variables|Default|GetPotionMesh))
  (bind _potionmesh_2 (Variables|Default|GetPotionMesh))
  (Utilities|FlowControl|Sequence
    (:then_0
      (Variables|Default|SetAScale (Transformation|GetActorScale3D))
      (Variables|Default|SetA (Transformation|GetWorldLocation (Variables|Default|GetPotionMesh)))
      (Utilities|FlowControl|Sequence
        (:then_0
          (bind _asbp_top_down_game_mode (Utilities|Casting|CastToBP_TopDownGameMode (Game|GetGameMode)))
          (if (== (Variables|/Game/StartContentStuff/TopDown/Blueprints/BP_TopDownGameMode.BP_TopDownGameMode_C|GetPotionsLeft _asbp_top_down_game_mode) 0)
            (bind _newtrack_0 (Timeline|Timeline PlayFromStart)
              (:Update
                (Transformation|SetRelativeLocation (Variables|Default|GetMeshMover) (Math|Vector|Lerp(Vector) "0, 0, 0" "0.000000,0.000000,200.000000" _newtrack_0) false false)
                (Transformation|SetActorScale3D (Math|Vector|Lerp(Vector) "0, 0, 0" (Variables|Default|GetAScale) _newtrack_0))))
            (else
              (bind _newtrack_0_2 (Timeline|RiseTL PlayFromStart)
                (:Update
                  (Transformation|SetRelativeLocation (Variables|Default|GetMeshMover) (Math|Vector|Lerp(Vector) "0, 0, 0" "0.000000,0.000000,200.000000" _newtrack_0_2) false false)
                  (Transformation|SetActorScale3D (Math|Vector|Lerp(Vector) "0, 0, 0" (Variables|Default|GetAScale) _newtrack_0_2)))))))
        (:then_1
          (bind _newtrack_1 (Timeline|SpinPotion_TL PlayFromStart)
            (:Update
              (Transformation|SetRelativeRotation _potionmesh (Math|Rotator|Lerp(Rotator) "0, 0, 0" "0.000000,-360.000000,0.000000" _newtrack_1) false false))
            (:Finished
              (Utilities|FlowControl|Sequence
                (:then_0
                  (Transformation|SetRelativeRotation _potionmesh "0, 0, 0" false false)
                  (Timeline|SpinPotion_TL PlayFromStart))))))))
    (:then_1
      (if (Variables|Default|GetRedTeamPotion?)
        (Rendering|Material|SetMaterial _potionmesh_2 0 "/Game/Models/Ingredients/BellPepper/bellpepperMeat.bellpepperMeat")
        (Utilities|FlowControl|Delay 0.3)
        (Effects|SpawnEmitteratLocation "/Game/StarterContent/Particles/P_RedPotion.P_RedPotion" (Transformation|GetWorldLocation (Variables|Default|GetPotionMesh)))
        (Components|StaticMesh|SetStaticMesh (Variables|Default|GetPotionMesh) "/Game/Models/Potions/EvilPotion.EvilPotion")
        (else
          (Rendering|Material|SetMaterial _potionmesh_2 0 "/Game/GhoulContent/Robe.Robe")
          (Utilities|FlowControl|Delay 0.3)
          (Effects|SpawnEmitteratLocation "/Game/StarterContent/Particles/P_GreenPotion.P_GreenPotion" (Transformation|GetWorldLocation (Variables|Default|GetPotionMesh))))))))

(fn ConstructionScript)