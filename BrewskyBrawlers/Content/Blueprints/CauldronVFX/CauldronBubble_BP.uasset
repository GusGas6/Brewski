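; Cauldron bubble VFX actor that rises briefly, then pops.
; On BeginPlay it randomizes its scale per axis and picks a random rise height.
; A timeline lerps the Sphere component's relative Z up to that height.
; When the timeline finishes, it spawns a small cauldron bang emitter at the sphere's location and destroys itself.
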(event EventBeginPlay
  (bind _returnvalue (Math|Random|RandomFloatinRange 0.8 1.4))
  (Transformation|SetActorScale3D (Math|Vector|MakeVector _returnvalue _returnvalue _returnvalue))
  (Variables|Default|SetBubbleHeight (Math|Random|RandomFloatinRange 4e+01 1.2e+02))
  (bind _newtrack_0 (Timeline|RaiseTL PlayFromStart)
    (:Update
      (Transformation|SetRelativeLocation (Variables|Default|GetSphere) (Math|Vector|Lerp(Vector) "0, 0, 0" (Math|Vector|MakeVector 0.0 0.0 (Variables|Default|GetBubbleHeight)) _newtrack_0) false false))
    (:Finished
      (Effects|SpawnEmitteratLocation "/Game/StarterContent/Particles/P_GoodCauldron_Bang.P_GoodCauldron_Bang" (Transformation|GetWorldLocation (Variables|Default|GetSphere)) "0, 0, 0" "0.050000,0.050000,0.050000")
      (Actor|DestroyActor))))

(fn ConstructionScript)