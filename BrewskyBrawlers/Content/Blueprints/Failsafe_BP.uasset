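; Failsafe volume actor that returns player characters to their starting position when they leave its overlap area.
; On ActorEndOverlap it tries casts in sequence to the third-person, second-person and first-person character Blueprints.
; The matching character teleports to its own stored InitialLocation or StartLocation, keeping its current rotation, and other actors are ignored.
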(event Collision|EventActorEndOverlap
  (params (OtherActor :type Actor%20Object%20Reference))
  (bind _asbp_third_person_character (Utilities|Casting|CastToBP_ThirdPersonCharacter OtherActor)
    (:then
      (Transformation|Teleport _asbp_third_person_character (Variables|/Game/ThirdPerson/Blueprints/BP_ThirdPersonCharacter.BP_ThirdPersonCharacter_C|GetInitialLocation _asbp_third_person_character) (Transformation|GetActorRotation _asbp_third_person_character)))
    (:CastFailed
      (bind _asbp_second_person_character (Utilities|Casting|CastToBP_SecondPerson_Character OtherActor)
        (:then
          (Transformation|Teleport _asbp_second_person_character (Variables|/Game/FirstPerson/Blueprints/BP_SecondPerson_Character.BP_SecondPerson_Character_C|GetStartLocation _asbp_second_person_character) (Transformation|GetActorRotation _asbp_second_person_character)))
        (:CastFailed
          (bind _asbp_first_person_character (Utilities|Casting|CastToBP_FirstPersonCharacter OtherActor))
          (Transformation|Teleport _asbp_first_person_character (Variables|/Game/FirstPerson/Blueprints/BP_FirstPersonCharacter.BP_FirstPersonCharacter_C|GetStartLocation _asbp_first_person_character) (Transformation|GetActorRotation _asbp_first_person_character)))))))

(fn ConstructionScript)