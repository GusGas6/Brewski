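; Collectible ghost essence pickup that the third-person character gathers by walking into it.
; A self-restarting timeline pulses the actor's scale and moves the essence component vertically for an idle bob.
; Sphere overlap with BP_ThirdPersonCharacter calls its PickupGhostEssence, spawns a small explosion particle at the essence and destroys the pickup.
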(event OnComponentBeginOverlap(Sphere)
  (params (OverlappedComponent :type Primitive%20Component%20Object%20Reference) (OtherActor :type Actor%20Object%20Reference) (OtherComp :type Primitive%20Component%20Object%20Reference) (OtherBodyIndex :type Integer) (bFromSweep :type Boolean) (SweepResult :type Hit%20Result%20Structure%20%28by%20ref%29))
  (bind _asbp_third_person_character (Utilities|Casting|CastToBP_ThirdPersonCharacter OtherActor))
  (Default|PickupGhostEssence _asbp_third_person_character 1)
  (Effects|SpawnEmitteratLocation "/Game/StarterContent/Particles/P_FlashbangExplosion.P_FlashbangExplosion" (Transformation|GetWorldLocation (Variables|Default|GetGhostEssence1)) "0, 0, 0" "0.400000,0.400000,0.400000")
  (Actor|DestroyActor))

(event EventBeginPlay
  (bind _newtrack_0 (Timeline|Timeline PlayFromStart)
    (:Update
      (Transformation|SetActorScale3D (Math|Vector|Lerp(Vector) "1.000000,1.000000,1.000000" "1.200000,1.200000,1.200000" _newtrack_0))
      (Transformation|SetRelativeLocation (Variables|Default|GetGhostEssence1) (Math|Vector|Lerp(Vector) "0.000000,0.000000,15.000000" "0.000000,0.000000,-15.000000" _newtrack_0) false false))
    (:Finished
      (Utilities|FlowControl|Sequence
        (:then_0
          (Timeline|Timeline PlayFromStart))))))

(fn ConstructionScript)