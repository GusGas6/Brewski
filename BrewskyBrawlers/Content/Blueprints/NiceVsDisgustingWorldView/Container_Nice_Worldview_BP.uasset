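; Container actor for the nice side of the nice-versus-disgusting worldview, shown as a shelf, table or chest.
; On BeginPlay it waits a tick, then sets its owner to the player character at OwnerIndex.
; After another tick it assigns the blockout static mesh matching ContainerEnum.
; The construction script is empty, so this mesh selection happens only at runtime.
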(event EventBeginPlay
  (Utilities|FlowControl|DelayUntilNextTick)
  (Actor|SetOwner (Game|GetPlayerCharacter (Variables|Default|GetOwnerIndex)))
  (Utilities|FlowControl|DelayUntilNextTick)
  (switch Utilities|FlowControl|Switch|SwitchonContainerEnum (Variables|Default|GetContainerEnum)
    (:NewEnumerator0
      (Components|StaticMesh|SetStaticMesh (Variables|Default|GetContainerMesh) "/Game/GustavTestFolder/_GENERATED/GustavSchrøder/ShelfBlockoutContainer.ShelfBlockoutContainer"))
    (:NewEnumerator1
      (Components|StaticMesh|SetStaticMesh (Variables|Default|GetContainerMesh) "/Game/GustavTestFolder/_GENERATED/GustavSchrøder/TableBlockoutContainer.TableBlockoutContainer"))
    (:NewEnumerator2
      (Components|StaticMesh|SetStaticMesh (Variables|Default|GetContainerMesh) "/Game/GustavTestFolder/_GENERATED/GustavSchrøder/ChestBlockoutContainer.ChestBlockoutContainer"))))

(fn ConstructionScript)