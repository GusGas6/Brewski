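; Ingredient respawner actor that brings a both-worlds ingredient back after a delay.
; RespawnIngredient stores the given transform, size and score ingredient type, then waits for RespawnDuration.
; It spawns an Ingredient_BothWorlds_BP with those stored values and destroys itself, so each respawner handles a single respawn.
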(event Custom|RespawnIngredient
  (params (Rotation :type Rotator) (Scale :type Vector) (Location :type Vector) (Size :type SizeEnum%20Enum :default "NewEnumerator0") (Ingredient :type IngredientEnum%20Enum :default "NewEnumerator0"))
  (Variables|Default|SetSpawn%20Transform%20Location Location)
  (Variables|Default|SetSpawn%20Transform%20Rotation Rotation)
  (Variables|Default|SetSpawn%20Transform%20Scale Scale)
  (Variables|Default|SetSize%20Enum Size)
  (Variables|Default|SetScore%20Ingredient%20Enum Ingredient)
  (Utilities|FlowControl|Delay (Variables|Default|GetRespawnDuration))
  (Game|SpawnActorfromClass "/Game/Blueprints/NiceVsDisgustingWorldView/Ingredient_BothWorlds_BP.Ingredient_BothWorlds_BP_C" (Math|Transform|MakeTransform (Variables|Default|GetSpawn%20Transform%20Location) (Variables|Default|GetSpawn%20Transform%20Rotation) (Variables|Default|GetSpawn%20Transform%20Scale)) "Undefined" "MultiplyWithRoot" 0 (Variables|Default|GetSize%20Enum) false (Variables|Default|GetScore%20Ingredient%20Enum) 0)
  (Actor|DestroyActor))

(fn ConstructionScript)