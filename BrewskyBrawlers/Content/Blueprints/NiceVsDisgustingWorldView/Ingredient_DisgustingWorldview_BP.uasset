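; Ingredient actor for the disgusting worldview, which gives itself an evil ingredient type and matching mesh based on its size.
; On BeginPlay it waits a tick, sets the player character at OwnerIndex as its owner, then waits another tick.
; It then switches on SizeEnum (small sphere, long capsule or large sphere) to set the type and DisgustingMesh.
; A random roll per size exists, but its visible branches select no distinct variant.
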(event EventBeginPlay
  (Utilities|FlowControl|DelayUntilNextTick)
  (Actor|SetOwner (Game|GetPlayerCharacter (Variables|Default|GetOwnerIndex)))
  (Utilities|FlowControl|DelayUntilNextTick)
  (switch Utilities|FlowControl|Switch|SwitchonSizeEnum (Variables|Default|GetSizeEnum)
    (:NewEnumerator0
      (switch int (Math|Random|RandomIntegerinRange 0 (Variables|Default|GetTotalAmountOfSmallSphere))
        (:Default
          _)
        (:0
          _))
      (Variables|Default|SetEvilIngredientEnum "NewEnumerator1")
      (Components|StaticMesh|SetStaticMesh (Variables|Default|GetDisgustingMesh) "/Game/GustavTestFolder/_GENERATED/GustavSchrøder/IngredientMeshSphereSmall_DisgustingVer.IngredientMeshSphereSmall_DisgustingVer"))
    (:NewEnumerator1
      (switch int (Math|Random|RandomIntegerinRange 0 (Variables|Default|GetTotalAmountOfLongCapsule))
        (:Default
          _)
        (:0
          _))
      (Variables|Default|SetEvilIngredientEnum "NewEnumerator2")
      (Components|StaticMesh|SetStaticMesh (Variables|Default|GetDisgustingMesh) "/Game/GustavTestFolder/_GENERATED/GustavSchrøder/IngredientMeshLargeCapsule_DisgustingVer.IngredientMeshLargeCapsule_DisgustingVer"))
    (:NewEnumerator2
      (switch int (Math|Random|RandomIntegerinRange 0 (Variables|Default|GetTotalAmountOfLargeSphere))
        (:Default
          _)
        (:0
          _))
      (Variables|Default|SetEvilIngredientEnum "NewEnumerator0")
      (Components|StaticMesh|SetStaticMesh (Variables|Default|GetDisgustingMesh) "/Game/GustavTestFolder/_GENERATED/GustavSchrøder/IngredientMeshSphereLarge_DisgustingVer.IngredientMeshSphereLarge_DisgustingVer"))))

(fn ConstructionScript)