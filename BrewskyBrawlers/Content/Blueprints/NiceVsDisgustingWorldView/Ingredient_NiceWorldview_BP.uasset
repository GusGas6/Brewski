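; Ingredient actor for the "nice" worldview that takes on a random food appearance when play begins.
; After one-tick delays around setting its owner to the player character at OwnerIndex, it switches on SizeEnum (small sphere, long capsule or large sphere).
; Each size rolls a random index within its own total, then sets the matching IngredientEnum and NiceMesh static mesh, with unmatched rolls falling back to that size's first entry.
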(event EventBeginPlay
  (bind _nicemesh (Variables|Default|GetNiceMesh))
  (bind _nicemesh_2 (Variables|Default|GetNiceMesh))
  (bind _nicemesh_3 (Variables|Default|GetNiceMesh))
  (Utilities|FlowControl|DelayUntilNextTick)
  (Actor|SetOwner (Game|GetPlayerCharacter (Variables|Default|GetOwnerIndex)))
  (Utilities|FlowControl|DelayUntilNextTick)
  (switch Utilities|FlowControl|Switch|SwitchonSizeEnum (Variables|Default|GetSizeEnum)
    (:NewEnumerator0
      (switch int (Math|Random|RandomIntegerinRange 0 (Variables|Default|GetTotalAmountOfSmallSphere))
        (:Default
          (Variables|Default|SetIngredientEnum "NewEnumerator1" :!label _label)
          (Components|StaticMesh|SetStaticMesh _nicemesh_2 "/Game/Models/Ingredients/Apple/SM_apple.SM_apple"))
        (:0
          (goto _label))
        (:1
          (Variables|Default|SetIngredientEnum "NewEnumerator12")
          (Components|StaticMesh|SetStaticMesh _nicemesh_2 "/Game/Models/Ingredients/Apple/SM_Apple2.SM_Apple2"))
        (:2
          (Variables|Default|SetIngredientEnum "NewEnumerator7")
          (Components|StaticMesh|SetStaticMesh _nicemesh_2 "/Game/Models/Ingredients/BellPepper/SM_BellpepperWhole.SM_BellpepperWhole"))
        (:3
          (Variables|Default|SetIngredientEnum "NewEnumerator4")
          (Components|StaticMesh|SetStaticMesh _nicemesh_2 "/Game/Models/Ingredients/Cherries/SM_cherries_CHERRY_LEAF.SM_cherries_CHERRY_LEAF"))
        (:4
          (Variables|Default|SetIngredientEnum "NewEnumerator8")
          (Components|StaticMesh|SetStaticMesh _nicemesh_2 "/Game/Models/Ingredients/Potato/SM_potato.SM_potato"))
        (:5
          (Variables|Default|SetIngredientEnum "NewEnumerator14")
          (Components|StaticMesh|SetStaticMesh _nicemesh_2 "/Game/Models/Ingredients/Pancakes/SM_pancakes.SM_pancakes"))
        (:6
          (Variables|Default|SetIngredientEnum "NewEnumerator15")
          (Components|StaticMesh|SetStaticMesh _nicemesh_2 "/Game/Models/Ingredients/Pancakes/SM_PanCakes__2_.SM_PanCakes__2_"))
        (:7
          (Variables|Default|SetIngredientEnum "NewEnumerator19")
          (Components|StaticMesh|SetStaticMesh _nicemesh_2 "/Game/Models/Ingredients/Metaballs/SM_Meatball.SM_Meatball"))))
    (:NewEnumerator1
      (switch int (Math|Random|RandomIntegerinRange 0 (Variables|Default|GetTotalAmountOfLongCapsule))
        (:Default
          (Variables|Default|SetIngredientEnum "NewEnumerator2" :!label _label_2)
          (Components|StaticMesh|SetStaticMesh _nicemesh_3 "/Game/Models/Ingredients/Cucumber/Cucumber_Cylinder_002.Cucumber_Cylinder_002"))
        (:0
          (goto _label_2))
        (:1
          (Variables|Default|SetIngredientEnum "NewEnumerator5")
          (Components|StaticMesh|SetStaticMesh _nicemesh_3 "/Game/Models/Ingredients/Bread/baguette.baguette"))
        (:2
          (Variables|Default|SetIngredientEnum "NewEnumerator6")
          (Components|StaticMesh|SetStaticMesh _nicemesh_3 "/Game/Models/Ingredients/Cherries/SM_carrot_carrot.SM_carrot_carrot"))
        (:3
          (Variables|Default|SetIngredientEnum "NewEnumerator11")
          (Components|StaticMesh|SetStaticMesh _nicemesh_3 "/Game/Models/Ingredients/Cucumber/Cucumber_Cylinder_002.Cucumber_Cylinder_002"))
        (:4
          (Variables|Default|SetIngredientEnum "NewEnumerator20")
          (Components|StaticMesh|SetStaticMesh _nicemesh_3 "/Game/Models/Ingredients/Candybar/SM_Candybar.SM_Candybar"))))
    (:NewEnumerator2
      (switch int (Math|Random|RandomIntegerinRange 0 (Variables|Default|GetTotalAmountOfLargeSphere))
        (:Default
          (Components|StaticMesh|SetStaticMesh _nicemesh "/Game/Models/Ingredients/Pumpkin/SM_jack-o-lantern.SM_jack-o-lantern" :!label _label_3)
          (Variables|Default|SetIngredientEnum "NewEnumerator10"))
        (:0
          (goto _label_3))
        (:1
          (Components|StaticMesh|SetStaticMesh _nicemesh "/Game/Models/Ingredients/Pumpkin/SM_Pumpkin.SM_Pumpkin")
          (Variables|Default|SetIngredientEnum "NewEnumerator0"))
        (:2
          (Components|StaticMesh|SetStaticMesh _nicemesh "/Game/Models/Ingredients/Bread/SM_Loaf.SM_Loaf")
          (Variables|Default|SetIngredientEnum "NewEnumerator13"))
        (:3
          (Components|StaticMesh|SetStaticMesh _nicemesh "/Game/Models/Ingredients/Coconut/SM_CocoNut.SM_CocoNut")
          (Variables|Default|SetIngredientEnum "NewEnumerator17"))
        (:4
          (Components|StaticMesh|SetStaticMesh _nicemesh "/Game/Models/Ingredients/Coconut/SM_HalfCocoNut.SM_HalfCocoNut")
          (Variables|Default|SetIngredientEnum "NewEnumerator18"))))))

(fn ConstructionScript)